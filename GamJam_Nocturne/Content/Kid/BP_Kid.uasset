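; BP_Kid is the kid actor, which drives the WBP_Nightmare widget it finds at BeginPlay.
; HitChild compares an image ID to the widget switcher's active index and, on a match, calls OnOf; the On/Of event triggers ChangeNightmare.
; Box overlaps query BPI_Scream actors for their object type, currently only printing debug text for Dog or Spider.
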(event `self.ReceiveBeginPlay`
  (bind _foundwidgets (`WidgetBlueprintLibrary.GetAllWidgetsOfClass` "/Game/Widgets/WBP_Nightmare.WBP_Nightmare_C" false))
  (set `self.As WBP_Nightmare` (`|GetArrayItem` _foundwidgets)))

(event `/Game/Lights/BPI_Interact.On/Of`
  (`/Game/Widgets/WBP_Nightmare.change Nightmare` (`self.As WBP_Nightmare`)))

(event `/Game/Kid/BPI_Child/BPI_HitChild.HitChild`
  (params (IdImage :type Integer))
  (if (== IdImage (`WidgetSwitcher.ActiveWidgetIndex` (`/Game/Widgets/WBP_Nightmare.WidgetSwitcher_138` (`self.As WBP_Nightmare`))))
    (`self.On/Of`)))

(event `self.Box.OnComponentBeginOverlap`
  (params (OverlappedComponent :type "PrimitiveComponent Object Reference") (OtherActor :type "Actor Object Reference") (OtherComp :type "PrimitiveComponent Object Reference") (OtherBodyIndex :type Integer) (bFromSweep :type Boolean) (SweepResult :type "HitResult Structure (by ref)"))
  (if (`KismetSystemLibrary.DoesImplementInterface` OtherActor "/Game/Characters/DelWork/BPI_Scream.BPI_Scream_C")
    (bind _objecttype (message `/Game/Characters/DelWork/BPI_Scream.GetObjectType` OtherActor))
    (switch `name` _objecttype
      (:`Dog`
        (`KismetSystemLibrary.PrintString` "Doggy!"))
      (:`Spider`
        (`KismetSystemLibrary.PrintString` "Spidy:")))))

(fn `UserConstructionScript`)