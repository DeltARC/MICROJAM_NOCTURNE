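; BP_KidBeton is a kid actor that plays a sleeping-baby sound on BeginPlay and screams when exposed to frightening objects.
; Box overlaps read the object type through BPI_Scream, then play the scream and set one of three notes by type on the first-person character's composition widget.
; A second box accepts BP_InteractableTape, playing a battle sound and destroying the tape before screaming and setting a note.
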(event `self.ReceiveBeginPlay`
  (`GameplayStatics.PlaySoundAtLocation` "/Game/SoundDesing/SoundE/361148__gutek__sleeping-baby-2yo-002_Cue.361148__gutek__sleeping-baby-2yo-002_Cue" (`self.K2_GetActorLocation`) (struct) 3.0 1.0 0.0 null null null null)
  (bind _foundwidgets (`WidgetBlueprintLibrary.GetAllWidgetsOfClass` "/Game/Widgets/WBP_Nightmare.WBP_Nightmare_C" false))
  (set `self.NewVar` (`|GetArrayItem` _foundwidgets))
  (bind _asbp_first_person_character (cast `/Game/FirstPerson/Blueprints/BP_FirstPersonCharacter` (`GameplayStatics.GetPlayerPawn` 0)))
  (set `self.As BP First Person Character` _asbp_first_person_character))

(event `self.Box.OnComponentBeginOverlap`
  (params (OverlappedComponent :type "PrimitiveComponent Object Reference") (OtherActor :type "Actor Object Reference") (OtherComp :type "PrimitiveComponent Object Reference") (OtherBodyIndex :type Integer) (bFromSweep :type Boolean) (SweepResult :type "HitResult Structure (by ref)"))
  (bind _aswbp_composition (`/Game/FirstPerson/Blueprints/BP_FirstPersonCharacter.AsWBP_Composition` (`self.As BP First Person Character`)))
  (if (`KismetSystemLibrary.DoesImplementInterface` OtherActor "/Game/Characters/DelWork/BPI_Scream.BPI_Scream_C")
    (bind _objecttype (message `/Game/Characters/DelWork/BPI_Scream.GetObjectType` OtherActor))
    (switch `name` _objecttype
      (:`Spider`
        (`GameplayStatics.PlaySoundAtLocation` "/Game/SoundDesing/SoundE/Scream_Cue.Scream_Cue" (`self.K2_GetActorLocation`) (struct) 1.0 2.0 0.0 null null null null)
        (`/Game/Widgets/WBP_CompositionMusique.SetNote` _aswbp_composition 0))
      (:`Dark`
        (`GameplayStatics.PlaySoundAtLocation` "/Game/SoundDesing/SoundE/Scream_Cue.Scream_Cue" (`self.K2_GetActorLocation`) (struct) 1.0 2.0 0.0 null null null null)
        (`/Game/Widgets/WBP_CompositionMusique.SetNote` _aswbp_composition 0))
      (:`Puppet`
        (`GameplayStatics.PlaySoundAtLocation` "/Game/SoundDesing/SoundE/Scream_Cue.Scream_Cue" (`self.K2_GetActorLocation`) (struct) 1.0 2.0 0.0 null null null null)
        (`/Game/Widgets/WBP_CompositionMusique.SetNote` _aswbp_composition 0))
      (:`Poop`
        (`GameplayStatics.PlaySoundAtLocation` "/Game/SoundDesing/SoundE/Scream_Cue.Scream_Cue" (`self.K2_GetActorLocation`) (struct) 1.0 1.0 0.0 null null null null)
        (`/Game/Widgets/WBP_CompositionMusique.SetNote` _aswbp_composition 1))
      (:`Water`
        (`GameplayStatics.PlaySoundAtLocation` "/Game/SoundDesing/SoundE/Scream_Cue.Scream_Cue" (`self.K2_GetActorLocation`) (struct) 1.0 1.0 0.0 null null null null)
        (`/Game/Widgets/WBP_CompositionMusique.SetNote` _aswbp_composition 1))
      (:`Dog`
        (`GameplayStatics.PlaySoundAtLocation` "/Game/SoundDesing/SoundE/Scream_Cue.Scream_Cue" (`self.K2_GetActorLocation`) (struct) 1.0 0.5 0.0 null null null null)
        (`/Game/Widgets/WBP_CompositionMusique.SetNote` _aswbp_composition 2))
      (:`Blood`
        (`GameplayStatics.PlaySoundAtLocation` "/Game/SoundDesing/SoundE/Scream_Cue.Scream_Cue" (`self.K2_GetActorLocation`) (struct) 1.0 0.5 0.0 null null null null)
        (`/Game/Widgets/WBP_CompositionMusique.SetNote` _aswbp_composition 2)))))

(event `self.Box1.OnComponentBeginOverlap`
  (params (OverlappedComponent :type "PrimitiveComponent Object Reference") (OtherActor :type "Actor Object Reference") (OtherComp :type "PrimitiveComponent Object Reference") (OtherBodyIndex :type Integer) (bFromSweep :type Boolean) (SweepResult :type "HitResult Structure (by ref)"))
  (cast `/Game/Characters/DelWork/BP_InteractableTape` OtherActor)
  (`GameplayStatics.PlaySoundAtLocation` "/Game/SoundDesing/SoundE/760104__gamexplosion__simple-battle-or-war_Cue.760104__gamexplosion__simple-battle-or-war_Cue" (`SceneComponent.K2_GetComponentLocation` (`self.Box1`)) (struct) 1.0 1.0 0.0 null null null null)
  (`self.K2_DestroyActor` OtherActor)
  (`GameplayStatics.PlaySoundAtLocation` "/Game/SoundDesing/SoundE/Scream_Cue.Scream_Cue" (`self.K2_GetActorLocation`) (struct) 1.0 1.0 0.0 null null null null)
  (`/Game/Widgets/WBP_CompositionMusique.SetNote` (`/Game/FirstPerson/Blueprints/BP_FirstPersonCharacter.AsWBP_Composition` (`self.As BP First Person Character`)) 1))

(fn `GetObjectType`
  (returns (ObjectType :type Name))
  (return "None"))

(fn `UserConstructionScript`)