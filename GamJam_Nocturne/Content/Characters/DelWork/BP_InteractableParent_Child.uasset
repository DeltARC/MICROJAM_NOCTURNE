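; Spider variant of the interactable parent Blueprint: a pawn that wanders around on its own and reports its object type as "Spider".
; BeginPlay starts a self-repeating Walk event that uses AI MoveTo toward a random reachable point near its current location, then waits a random short delay, whether the move succeeds or fails.
; The parent BeginPlay call is disabled, and the Roam function is empty.
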(event `self.ReceiveBeginPlay`
  (`self.Walk`))

(event `Walk`
  (`|AIMoveTo` self (`NavigationSystemV1.K2_GetRandomReachablePointInRadius` (`self.K2_GetActorLocation`) 100.0 null null) null
    (:`OnSuccess`
      _)
    (:`OnFail`
      _))
  (`KismetSystemLibrary.Delay` (`KismetMathLibrary.RandomFloatInRange` 1.0 3.0))
  (`self.Walk`))

(fn `GetObjectType`
  (returns (ObjectType :type Name))
  (return "Spider"))

(fn `Roam`)

(fn `UserConstructionScript`
  (`parent.UserConstructionScript`))