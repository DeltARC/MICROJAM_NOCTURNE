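; BP_InteractableDog is a dog that wanders the level on its own and occasionally leaves poop behind.
; From BeginPlay, Roam loops endlessly: AIMoveTo a random reachable point nearby, wait briefly, then roam again, whether the move succeeded or failed.
; As each new move begins, a random roll may spawn BP_InteractablePoop at the dog's transform.
; GetObjectType identifies it as "Dog", and the WALK function is an empty stub.
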(event `self.ReceiveBeginPlay`
  (`self.Roam`))

(event `Roam`
  (`|AIMoveTo` self (`NavigationSystemV1.K2_GetRandomReachablePointInRadius` (`self.K2_GetActorLocation`) 1000.0 null null) null
    (:`OnSuccess`
      _)
    (:`OnFail`
      _))
  (`KismetSystemLibrary.Delay` (`KismetMathLibrary.RandomFloatInRange` 1.0 3.0))
  (`self.Roam`)
  (if (== (`KismetMathLibrary.RandomIntegerInRange` 1 8) 7)
    (`|SpawnActorFromClass` "/Game/Characters/DelWork/BP_InteractablePoop.BP_InteractablePoop_C" (`self.GetTransform`) "Undefined" "MultiplyWithRoot" null null)))

(fn `GetObjectType`
  (returns (ObjectType :type Name))
  (return "Dog"))

(fn `UserConstructionScript`
  (`parent.UserConstructionScript`))

(fn `wALK`)