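; Interactable pickup, likely a parent class, that the first-person player grabs and carries in the right hand.
; Interact applies HeldSprite to the hand, stores the item as held on the player and teleports its capsule to a fixed spot instead of destroying it.
; A chain of HeldSprite material comparisons identifies items like spider, dog or ketchup, playing each one's sound plus a dialogue widget line gated once by a flag.
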(event `self.ReceiveBeginPlay`)

(event `/Game/Characters/DelWork/BPI_Interaction.Interact`
  (params (Player_Ref :type "Character Object Reference"))
  (bind _asbp_first_person_character (cast `/Game/FirstPerson/Blueprints/BP_FirstPersonCharacter` Player_Ref))
  ; Set la main au bon sprite
  (`PrimitiveComponent.SetMaterial` (`/Game/FirstPerson/Blueprints/BP_FirstPersonCharacter.RightHand` _asbp_first_person_character) 0 (`self.HeldSprite`))
  (`|ExecutionSequence`
    (:`then_0`
      (if (== (`self.HeldSprite`) "/Game/Characters/DelWork/HandSprite/Spider_Hand_Mat.Spider_Hand_Mat")
        (`GameplayStatics.PlaySound2D` "/Game/SoundDesing/SoundE/238147__m4d3r0__tiny-insectrat-2-3-pitches.238147__m4d3r0__tiny-insectrat-2-3-pitches" 1.0 1.1 0.0 null null)
        (if (not (`self.AJouerSpider`))
          (bind _returnvalue (`|CreateWidget` "/Game/Widgets/WBP_DialogueBox.WBP_DialogueBox_C"))
          (bind _output_get (set `self.DialogueSpider` _returnvalue))
          (`UserWidget.AddToViewport` _output_get 0)
          (`/Game/Widgets/WBP_DialogueBox.UpdateText` _output_get "No, no, don't bite me, save your venom for the little one.")
          (set `self.AJouerSpider` true)))
      ; Garde en mémoire l'item que le joueur a attrapé
      (set `/Game/FirstPerson/Blueprints/BP_FirstPersonCharacter.ItemHolded` self _asbp_first_person_character :!label _label)
      (`SceneComponent.K2_SetWorldLocation` (`self.CapsuleComponent`) (2000.0 2000.0 20.0) false true)
      (set `/Game/FirstPerson/Blueprints/BP_FirstPersonCharacter.IsHoldingSomething?` true _asbp_first_person_character))
    (:`then_1`
      (if (== (`self.HeldSprite`) "/Game/Characters/DelWork/HandSprite/T_dog_hand_Mat.T_dog_hand_Mat")
        (`GameplayStatics.PlaySound2D` "/Game/SoundDesing/SoundE/418108__crazymonke9__dog-tripple-bark.418108__crazymonke9__dog-tripple-bark" 1.0 1.1 0.0 null null)
        (if (`self.AJouerDog`)
          (goto _label)
          (else
            (bind _returnvalue_2 (`|CreateWidget` "/Game/Widgets/WBP_DialogueBox.WBP_DialogueBox_C"))
            (bind _output_get_2 (set `self.DialogueDog` _returnvalue_2))
            (`UserWidget.AddToViewport` _output_get_2 0)
            (`/Game/Widgets/WBP_DialogueBox.UpdateText` _output_get_2 "Shh, stop barking, you're going to wake him up.")
            (set `self.AJouerDog` true)
            (goto _label)))
        (else
          (goto _label))))
    (:`then_2`
      (if (== (`self.HeldSprite`) "/Game/Characters/DelWork/HandSprite/Tomato_hand_Mat.Tomato_hand_Mat")
        (`GameplayStatics.PlaySound2D` "/Game/SoundDesing/SoundE/814842__designerschoice__toonsplt-samsung-galaxy-smartphone-cu_squirt-ketchup-bottle_nicholas-judy_tdc.814842__designerschoice__toonsplt-samsung-galaxy-smartphone-cu_squirt-ketchup-bottle_nicholas-judy_tdc" 1.0 1.1 0.0 null null)
        (if (`self.AJouerKetchup`)
          (goto _label)
          (else
            (bind _returnvalue_3 (`|CreateWidget` "/Game/Widgets/WBP_DialogueBox.WBP_DialogueBox_C"))
            (bind _output_get_3 (set `self.DialogueKetchup` _returnvalue_3))
            (`UserWidget.AddToViewport` _output_get_3 0)
            (`/Game/Widgets/WBP_DialogueBox.UpdateText` _output_get_3 "I wish it was real blood, school's rules are so annoying...")
            (set `self.AJouerKetchup` true)
            (goto _label)))))
    (:`then_3`
      (if (== (`self.HeldSprite`) "/Game/Characters/DelWork/HandSprite/Tape_hand_Mat.Tape_hand_Mat")
        (`GameplayStatics.PlaySound2D` "/Game/SoundDesing/SoundE/652389__department64__cassette-tape-rattle-63.652389__department64__cassette-tape-rattle-63" 1.0 1.0 0.0 null null)
        (if (`self.AJouerTape`)
          (goto _label)
          (else
            (bind _returnvalue_4 (`|CreateWidget` "/Game/Widgets/WBP_DialogueBox.WBP_DialogueBox_C"))
            (bind _output_get_4 (set `self.DialogueTape` _returnvalue_4))
            (`UserWidget.AddToViewport` _output_get_4 0)
            (`/Game/Widgets/WBP_DialogueBox.UpdateText` _output_get_4 "Ahh good old time memories... Almost forgot about my bombing test next week")
            (set `self.AJouerTape` true)
            (goto _label)))))
    (:`then_4`
      (if (== (`self.HeldSprite`) "/Game/Characters/DelWork/HandSprite/Water_hand_Mat.Water_hand_Mat")
        (`GameplayStatics.PlaySound2D` "/Game/SoundDesing/SoundE/255670__spectral9__wine-glass-hit-f6.255670__spectral9__wine-glass-hit-f6" 1.0 1.0 0.0 null null)
        (if (`self.AJouerWater`)
          (goto _label)
          (else
            (bind _returnvalue_5 (`|CreateWidget` "/Game/Widgets/WBP_DialogueBox.WBP_DialogueBox_C"))
            (bind _output_get_5 (set `self.DialogueWater` _returnvalue_5))
            (`UserWidget.AddToViewport` _output_get_5 0)
            (`/Game/Widgets/WBP_DialogueBox.UpdateText` _output_get_5 "Ouhh fake pipi, this score is gonna be peak !")
            (set `self.AJouerWater` true)
            (goto _label)))))
    (:`then_5`
      (if (== (`self.HeldSprite`) "/Game/Characters/DelWork/HandSprite/Poop_Hand_Mat.Poop_Hand_Mat")
        (`GameplayStatics.PlaySound2D` "/Game/SoundDesing/SoundE/446000__breviceps__fart-3.446000__breviceps__fart-3" 1.0 1.0 0.0 null null)
        (if (`self.AJouerPoop`)
          (goto _label)
          (else
            (bind _returnvalue_6 (`|CreateWidget` "/Game/Widgets/WBP_DialogueBox.WBP_DialogueBox_C"))
            (bind _output_get_6 (set `self.DialoguePoop` _returnvalue_6))
            (`UserWidget.AddToViewport` _output_get_6 0)
            (`/Game/Widgets/WBP_DialogueBox.UpdateText` _output_get_6 "Ouhhh shii makes my mouth watering hmmm")
            (set `self.AJouerPoop` true)
            (goto _label)))))))

(fn `UserConstructionScript`)