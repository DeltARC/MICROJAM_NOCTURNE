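; Light bulb actor that can be switched on and off in the level.
; Its On/Of custom event uses a FlipFlop to set the OnOff flag, alternating the state on each call.
; Each state flips the Cube's rotation, sets the SpotLight intensity and swaps the Ampoule material between black and glowing yellow, with the first call turning the light off.
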(event `/Game/Lights/BPI_Interact.On/Of`
  ; Permet d'allumer ou d'éteindre la lumier
  (bind _isa (`/Engine/EditorBlueprintResources/StandardMacros.FlipFlop`)
    (:`A`
      _)
    (:`B`
      _))
  (bind _output_get (set `self.On/Off` _isa))
  (if _output_get
    (`SceneComponent.K2_SetRelativeRotation` (`self.Cube`) (struct :`Yaw` 180.0) false false)
    (`LightComponent.SetIntensity` (`self.SpotLight`) 0.0)
    (`PrimitiveComponent.SetMaterial` (`self.Ampoule`) 0 "/Game/StarterContent/Blueprints/Assets/M_LightStage_Skybox_Black.M_LightStage_Skybox_Black")
    (else
      (`SceneComponent.K2_SetRelativeRotation` :`self` (`self.Cube`))
      (`LightComponent.SetIntensity` (`self.SpotLight`) 1000.0)
      (`PrimitiveComponent.SetMaterial` (`self.Ampoule`) 0 "/Game/Lights/Materials/M_YellowLight.M_YellowLight"))))

(fn `UserConstructionScript`)