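; BP_Object_Dady_Child is an object Blueprint that reports physical hits on its Cube component to the actors it collides with.
; On a component hit it ignores BP_Kid actors and sends HitChildMessage with its Id to any other actor implementing BPI_HitChild.
; The interface message is its only active logic, so receivers decide how to respond to the hit.
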(event `self.Cube.OnComponentHit`
  (params (HitComponent :type "PrimitiveComponent Object Reference") (OtherActor :type "Actor Object Reference") (OtherComp :type "PrimitiveComponent Object Reference") (NormalImpulse :type "Vector Structure") (Hit :type "HitResult Structure (by ref)"))
  (cast `/Game/Kid/BP_Kid` OtherActor
    (:`CastFailed`
      (if (`KismetSystemLibrary.DoesImplementInterface` OtherActor "/Game/Kid/BPI_Child/BPI_HitChild.BPI_HitChild_C")
        (message `/Game/Kid/BPI_Child/BPI_HitChild.HitChild` OtherActor (`self.Id`))))))

(fn `UserConstructionScript`
  (`parent.UserConstructionScript`))